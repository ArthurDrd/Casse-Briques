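; Player controller that drives the bat pawn with mouse movement in what appears to be a brick-breaker game.
; On possess, it casts and caches the bat pawn.
; The mouse axis, scaled by sensitivity, selects right, left or stop on the pawn by its sign.
; When moving, the scaled value also feeds the pawn's play rate, so mouse speed controls bat speed.
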(event `self.ReceivePossess`
  (params (PossessedPawn :type "Pawn Object Reference"))
  ;[0.3503 1 0.4705] On possess
  (bind _asb_pawn_bat (cast `/Game/CasseBriqueContent/Blueprints/B_Pawn_Bat` PossessedPawn))
  (set `self.As B Pawn Bat` _asb_pawn_bat))

(event `InputAxis|Move - Mouse`
  (params (AxisValue :type "Float (single-precision)"))
  (bind _as_b_pawn_bat (`self.As B Pawn Bat`))
  (bind _mouve_move_rate (`self.Mouve Move Rate`))
  ;[1 0.3372 0.9979] Move Bat
  (bind _output_get (set `self.Mouve Move Rate` (* AxisValue (`self.Mouse Sensitivity`))))
  (`/Engine/EditorBlueprintResources/StandardMacros.CompareFloat` _output_get
    (:`>`
      (`/Game/CasseBriqueContent/Blueprints/B_Pawn_Bat.Move Right` _as_b_pawn_bat)
      (`/Game/CasseBriqueContent/Blueprints/B_Pawn_Bat.Set Play Rate` _as_b_pawn_bat _mouve_move_rate :!label _label))
    (:`==`
      (`/Game/CasseBriqueContent/Blueprints/B_Pawn_Bat.Stop Moving` _as_b_pawn_bat))
    (:`<`
      (`/Game/CasseBriqueContent/Blueprints/B_Pawn_Bat.Move Left` _as_b_pawn_bat)
      (`/Engine/EditorBlueprintResources/StandardMacros.NegateFloat` _mouve_move_rate
        (:`  `
          (goto _label))))))

(fn `UserConstructionScript`)