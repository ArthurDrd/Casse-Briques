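; B_Pawn_Bat is the player bat pawn for a brick-breaker game, sliding along a spline to move left and right.
; A timeline outputs a normalized spline position, which places BatAnchor at that world location with sweep enabled.
; Movement events play, reverse or stop the timeline, so its play rate sets bat speed.
; ResetBat sets the timeline time on BeginPlay or when called.
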(event `self.ReceiveBeginPlay`
  ;[1 1 1] Setup
  (`self.Reset Bat`))

(event `Set Play Rate`
  (params (NewRate :type "Float (single-precision)"))
  ;[1 1 1] Bat Speed
  (`TimelineComponent.SetPlayRate` (`self.Timeline Move Bat`) NewRate))

(event `Move Right`
  (bind _spline (`self.Spline`))
  ;[0 0.8189 1] Move Bat
  (bind (_direction _bat_position_on_spline) (`Timeline|Timeline Move Bat` :`NewTime` 0.5 :!label _label)
    (:`Update`
      (bind _returnvalue_location (`KismetMathLibrary.BreakTransform` (`SplineComponent.GetTransformAtDistanceAlongSpline` _spline (* (`SplineComponent.GetSplineLength` _spline) _bat_position_on_spline) "World" false)))
      (`SceneComponent.K2_SetWorldTransform` (`self.BatAnchor`) (`KismetMathLibrary.MakeTransform` _returnvalue_location) true false))))

(event `Stop Moving`
  ;[0 0.8189 1] Move Bat
  (goto _label :!via `Stop`))

(event `Move Left`
  ;[0 0.8189 1] Move Bat
  (goto _label :!via `Reverse`))

(event `Reset Bat`
  ;[0 0.8189 1] Move Bat
  (goto _label :!via `SetNewTime`))

(fn `UserConstructionScript`)